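; BP_PhoneRing is an interactable phone that rings when triggered and plays a scripted one-time call when answered.
; TriggerPhone activates the ringing audio component, and the first Interact destroys it.
; A chain of timed delays then plays connection, voice and static clips as 2D sounds through to the hang-up.
; The sequence ends by calling LeadTowardsTrials on BP_LeadToFinalNoteInHouse to move the player's objective on.
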(event `TriggerPhone`
  (`ActorComponent.SetActive` (`self.Audio`) true false))

(event `/Game/LD24_VinterCollab/Blueprints/Interfaces/BPI_Interact.Interact`
  (`/Engine/EditorBlueprintResources/StandardMacros.DoOnce` false
    (:`Completed`
      (`ActorComponent.K2_DestroyComponent` (`self.Audio`))
      (`GameplayStatics.PlaySound2D` "/Game/Dialouge/Helper/connection.connection" 1.0 1.0 0.0 null null)
      (`KismetSystemLibrary.Delay` 8.2)
      (`GameplayStatics.PlaySound2D` "/Game/Dialouge/Helper/wayout.wayout" 1.0 1.0 0.0 null null)
      (`KismetSystemLibrary.Delay` 4.3)
      (`GameplayStatics.PlaySound2D` "/Game/Sound/35291__jace__continuous-static.35291__jace__continuous-static" 1.0 1.0 0.0 null null)
      (`KismetSystemLibrary.Delay` 6.2)
      (`GameplayStatics.PlaySound2D` "/Game/Dialouge/BadGuy/expecting.expecting" 1.0 1.0 0.0 null null)
      (`KismetSystemLibrary.Delay` 3.0)
      (`GameplayStatics.PlaySound2D` "/Game/Dialouge/BadGuy/foolish.foolish" 1.0 1.0 0.0 null null)
      (`KismetSystemLibrary.Delay` 12.2)
      (`GameplayStatics.PlaySound2D` "/Game/Dialouge/BadGuy/trials.trials" 1.0 1.0 0.0 null null)
      (`KismetSystemLibrary.Delay` 17.0)
      (`GameplayStatics.PlaySound2D` "/Game/Sound/hnag_up.hnag_up" 1.0 1.0 0.0 null null)
      (bind _returnvalue (`GameplayStatics.GetActorOfClass` "/Game/LD24_VinterCollab/Blueprints/Objectives/HouseOnFloatingIsland/BP_LeadToFinalNoteInHouse.BP_LeadToFinalNoteInHouse_C"))
      (`/Game/LD24_VinterCollab/Blueprints/Objectives/HouseOnFloatingIsland/BP_LeadToFinalNoteInHouse.LeadTowardsTrials` _returnvalue))))

(fn `UserConstructionScript`)
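; Door actor that slides open while three pressure plate flags are all true.
; Tick checks the flags, playing a timeline that lerps the door from its starting position by a move offset, or reversing it otherwise.
; The light switches to M_Bullet when all are set and never switches back.
; A separate OpenDoor event does the same slide on its own timeline; its call in this graph is unwired.
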(event `self.ReceiveBeginPlay`
  (set `self.originalPos` (`SceneComponent.RelativeLocation` (`self.Door`))))

(event `self.ReceiveTick`
  (params (DeltaSeconds :type "Float (single-precision)"))
  (bind _originalpos (`self.originalPos`))
  (if (and (`self.plateOne`) (`self.plateTwo`) (`self.plateThree`))
    (`PrimitiveComponent.SetMaterial` (`self.Light`) 0 "/Game/LD24_VinterCollab/Materials/M_Bullet.M_Bullet")
    (bind (_direction _progress) (`Timeline|Timeline` :!label _label)
      (:`Update`
        (`SceneComponent.K2_SetRelativeLocation` (`self.Door`) (`KismetMathLibrary.VLerp` _originalpos (- _originalpos (`self.doorMoveAmount`)) _progress) false false)))
    (else
      (goto _label :!via `Reverse`))))

(event `OpenDoor`
  (bind _originalpos (`self.originalPos`))
  (bind (_direction _progress) (`Timeline|Open Door T`)
    (:`Update`
      (`SceneComponent.K2_SetRelativeLocation` (`self.Door`) (`KismetMathLibrary.VLerp` _originalpos (- _originalpos (`self.doorMoveAmount`)) _progress) false false))))

(fn `UserConstructionScript`)
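; BP_Sword is an interactable sword pickup that acts as a navigation objective and story trigger.
; On BeginPlay it sets the first-person character's NavPoint to its own location.
; Interact tells the player to pick up the sword, asks BP_Objective for a new nav point, destroys the sword actor and makes BP_Phone ring.
; The objective and phone are found at runtime by class lookup.
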(event `self.ReceiveBeginPlay`
  (bind _asbp_first_person_character (cast `/Game/FirstPerson/Blueprints/BP_FirstPersonCharacter` (`GameplayStatics.GetPlayerCharacter` 0)))
  (set `/Game/FirstPerson/Blueprints/BP_FirstPersonCharacter.NavPoint` (`self.K2_GetActorLocation`) _asbp_first_person_character))

(event `/Game/LD24_VinterCollab/Blueprints/Interfaces/BPI_Interact.Interact`
  (bind _asbp_first_person_character (cast `/Game/FirstPerson/Blueprints/BP_FirstPersonCharacter` (`GameplayStatics.GetPlayerCharacter` 0)))
  (`/Game/FirstPerson/Blueprints/BP_FirstPersonCharacter.PickUpSword` _asbp_first_person_character)
  (bind _returnvalue (`GameplayStatics.GetActorOfClass` "/Game/LD24_VinterCollab/Blueprints/BP_Objective.BP_Objective_C"))
  (`/Game/LD24_VinterCollab/Blueprints/BP_Objective.NewNavPoint` _returnvalue)
  (`self.K2_DestroyActor`)
  (bind _returnvalue_2 (`GameplayStatics.GetActorOfClass` "/Game/LD24_VinterCollab/Blueprints/BP_Phone.BP_Phone_C"))
  (`/Game/LD24_VinterCollab/Blueprints/BP_Phone.Phone Ring` _returnvalue_2))

(fn `UserConstructionScript`)
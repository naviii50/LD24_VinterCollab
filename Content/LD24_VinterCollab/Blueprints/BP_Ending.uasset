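; BP_Ending is an interactable phone actor that runs the game's ending sequence.
; The PhoneRinging event plays a ringing sound from its audio component, moved to the actor's location.
; Interact stops the ringing and, through a DoOnce, plays a 2D sound, then after timed delays shows the WBP_TheEnd widget and opens the main menu level.
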(event `Phone Ringing`
  (bind _audio (`self.Audio`))
  ;[1 1 1] Phone Rings
  (`AudioComponent.SetSound` _audio "/Game/Sound/phone_ringing.phone_ringing")
  (`AudioComponent.Play` _audio 0.0)
  (`SceneComponent.K2_SetWorldLocation` _audio (`self.K2_GetActorLocation`) false false))

(event `self.Interact`
  ;[1 1 1] Phone Stops Ringing
  (`AudioComponent.Stop` (`self.Audio`))
  ;[1 1 1] Voiceline ?
  (`/Engine/EditorBlueprintResources/StandardMacros.DoOnce` false
    (:`Completed`
      (`GameplayStatics.PlaySound2D` null 1.0 1.0 0.0 null null)
      ;[1 1 1] Delay Before Fade ?
      (`KismetSystemLibrary.Delay` 10.0)
      ;[1 1 1] Fade to End Screen
      (bind _returnvalue (`|CreateWidget` "/Game/Tiger/UI/WBP_TheEnd.WBP_TheEnd_C"))
      (`UserWidget.AddToViewport` _returnvalue 0)
      ;[1 1 1] Opens Main Menu
      (`KismetSystemLibrary.Delay` 11.0)
      (`GameplayStatics.OpenLevelBySoftObjectPtr` "/Game/MainMenu/MainMenuLevel.MainMenuLevel"))))

(fn `UserConstructionScript`)
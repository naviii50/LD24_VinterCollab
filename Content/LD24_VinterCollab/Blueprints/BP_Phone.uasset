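; BP_Phone is an interactable phone that plays a one-time call, then hands the player on to the boat.
; PhoneRing activates the audio and sets the character's NavPoint to the phone, only if the player has the sword.
; Interact stops the ring and plays timed 2D voice clips that branch on HasSword.
; After the hang-up sound, it destroys itself and calls LeadToBoat on BP_WoddenBoat.
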(event `Phone Ring`
  (bind _asbp_first_person_character (cast `/Game/FirstPerson/Blueprints/BP_FirstPersonCharacter` (`GameplayStatics.GetPlayerCharacter` 0)))
  (if (`/Game/FirstPerson/Blueprints/BP_FirstPersonCharacter.hasSword` _asbp_first_person_character)
    (`ActorComponent.SetActive` (`self.Audio`) true false)
    (set `/Game/FirstPerson/Blueprints/BP_FirstPersonCharacter.NavPoint` (`self.K2_GetActorLocation`) _asbp_first_person_character)))

(event `/Game/LD24_VinterCollab/Blueprints/Interfaces/BPI_Interact.Interact`
  (`/Engine/EditorBlueprintResources/StandardMacros.DoOnce` false
    (:`Completed`
      (`ActorComponent.K2_DestroyComponent` (`self.Audio`))
      (`GameplayStatics.PlaySound2D` "/Game/Dialouge/Helper/mr_mid_intro.mr_mid_intro" 1.0 1.0 0.0 null null)
      (bind _asbp_first_person_character (cast `/Game/FirstPerson/Blueprints/BP_FirstPersonCharacter` (`GameplayStatics.GetPlayerCharacter` 0)))
      (if (`/Game/FirstPerson/Blueprints/BP_FirstPersonCharacter.hasSword` _asbp_first_person_character)
        (`KismetSystemLibrary.Delay` 8.5)
        (`GameplayStatics.PlaySound2D` "/Game/Dialouge/Helper/hasSwordTrue.hasSwordTrue" 1.0 1.0 0.0 null null)
        (else
          (`KismetSystemLibrary.Delay` 8.5)
          (`GameplayStatics.PlaySound2D` "/Game/Dialouge/Helper/hasSwordFalse.hasSwordFalse" 1.0 1.0 0.0 null null)))
      (`KismetSystemLibrary.Delay` 6.1)
      (`GameplayStatics.PlaySound2D` "/Game/Sound/hnag_up.hnag_up" 1.0 1.0 0.0 null null)
      (`self.K2_DestroyActor`)
      (bind _returnvalue (`GameplayStatics.GetActorOfClass` "/Game/LD24_VinterCollab/Blueprints/Objectives/HouseOnFloatingIsland/BP_WoddenBoat.BP_WoddenBoat_C"))
      (`/Game/LD24_VinterCollab/Blueprints/Objectives/HouseOnFloatingIsland/BP_WoddenBoat.LeadToBoat` _returnvalue)
      (`self.K2_DestroyActor`))))

(fn `UserConstructionScript`)
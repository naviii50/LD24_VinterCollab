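; BP_NoteMaker is a world note pickup that lets the player open and close a note card on screen while overlapping it.
; Overlap begin enables input and writes its NoteCard value to the first-person character's NoteCardIndex.
; Interact plays a pickup sound and uses a FlipFlop to create or remove WBP_NoteCardDisplay.
; Overlap end disables input and removes any open cards without resetting the FlipFlop.
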(event `/Game/LD24_VinterCollab/Blueprints/Interfaces/BPI_Interact.Interact`
  (`GameplayStatics.PlaySound2D` "/Game/Sound/428665__jomse__pickupbook2.428665__jomse__pickupbook2" 1.0 1.0 0.0 null null)
  (`/Engine/EditorBlueprintResources/StandardMacros.FlipFlop`
    (:`A`
      (bind _returnvalue (`|CreateWidget` "/Game/LD24_VinterCollab/Blueprints/NoteSystem/WBP_NoteCardDisplay.WBP_NoteCardDisplay_C"))
      (`UserWidget.AddToViewport` _returnvalue 0))
    (:`B`
      (bind _foundwidgets (`WidgetBlueprintLibrary.GetAllWidgetsOfClass` "/Game/LD24_VinterCollab/Blueprints/NoteSystem/WBP_NoteCardDisplay.WBP_NoteCardDisplay_C" :!label _label))
      (`Widget.RemoveFromParent` _foundwidgets))))

(event `self.ReceiveActorEndOverlap`
  (params (OtherActor :type "Actor Object Reference"))
  (`self.DisableInput` null)
  (goto _label))

(event `self.ReceiveActorBeginOverlap`
  (params (OtherActor :type "Actor Object Reference"))
  (`self.EnableInput` (`GameplayStatics.GetPlayerController` 0))
  (bind _asbp_first_person_character (cast `/Game/FirstPerson/Blueprints/BP_FirstPersonCharacter` (`GameplayStatics.GetPlayerCharacter` 0)))
  (set `/Game/FirstPerson/Blueprints/BP_FirstPersonCharacter.NoteCardIndex` (`self.NoteCard`) _asbp_first_person_character))

(fn `UserConstructionScript`)
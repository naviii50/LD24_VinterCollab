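; BP_Boss is a boss character for a boss fight, with health, a health bar widget and a montage attack.
; Damage events reduce health, and at zero the boss stops moving and its mesh switches to physics simulation.
; Tick pushes health to the widget created at BeginPlay.
; Bullets overlapping the capsule are destroyed without applying damage here, and Attack uses a flag to avoid restarting its montage.
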(event `self.CapsuleComponent.OnComponentBeginOverlap`
  (params (OverlappedComponent :type "PrimitiveComponent Object Reference") (OtherActor :type "Actor Object Reference") (OtherComp :type "PrimitiveComponent Object Reference") (OtherBodyIndex :type Integer) (bFromSweep :type Boolean) (SweepResult :type "HitResult Structure (by ref)"))
  (bind _asbp_bulet (cast `/Game/Alvin/BP/BP_Bulet` OtherActor))
  (`self.K2_DestroyActor` _asbp_bulet))

(event `/Game/LD24_VinterCollab/Blueprints/Interfaces/BPI_Damage.Damage`
  (set `self.Health` (- (`self.Health`) 5.0))
  (if (<= (`self.Health`) 0.0)
    (`CharacterMovementComponent.DisableMovement` (`self.CharacterMovement`))
    (`PrimitiveComponent.SetSimulatePhysics` (`self.Mesh`) true)))

(event `self.ReceiveBeginPlay`
  (bind _returnvalue (`|CreateWidget` "/Game/Filip/BossFight/WB_BossFightHealth.WB_BossFightHealth_C"))
  (`UserWidget.AddToViewport` _returnvalue 0)
  (set `self.Health UI` _returnvalue))

(event `self.ReceiveTick`
  (params (DeltaSeconds :type "Float (single-precision)"))
  (`ProgressBar.SetPercent` (`/Game/Filip/BossFight/WB_BossFightHealth.HealthBar` (`self.Health UI`)) (/ (`self.Health`) 100.0)))

(event `/Game/Filip/BossFight/BPI_Bossfight.Attack`
  ;[1 1 1] Attack
  (if (not (`self.isAttacking`))
    (`|PlayMontage` (`self.Mesh`) "/Game/Filip/Ancient_Golem/Demo/ThirdPersonJump_Start_Montage.ThirdPersonJump_Start_Montage"
      (:`then`
        (set `self.isAttacking` true))
      (:`OnCompleted`
        (set `self.isAttacking` false)))))

(fn `UserConstructionScript`)
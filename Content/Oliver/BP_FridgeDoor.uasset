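; BP_FridgeDoor is an interactable fridge door that the player opens with the E key and that closes itself.
; A box overlap with the first-person character sets a proximity flag, shows an interact widget and turns on a point light, reversing all three on exit.
; A timeline lerps the door's relative rotation toward 90 degrees, and a Delay on its Update pin later triggers CloseDoorFridge to reverse it.
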(event `self.ReceiveBeginPlay`
  (`self.EnableInput` (`GameplayStatics.GetPlayerController` 0))
  (`SceneComponent.SetVisibility` (`self.PointLight`) false false))

(event `self.Box.OnComponentBeginOverlap`
  (params (OverlappedComponent :type "PrimitiveComponent Object Reference") (OtherActor :type "Actor Object Reference") (OtherComp :type "PrimitiveComponent Object Reference") (OtherBodyIndex :type Integer) (bFromSweep :type Boolean) (SweepResult :type "HitResult Structure (by ref)"))
  (cast `/Game/FirstPerson/Blueprints/BP_FirstPersonCharacter` OtherActor)
  (set `self.IsplayerNear?` true)
  (bind _returnvalue (`|CreateWidget` "/Game/Oliver/Widgets/WBP_Interact.WBP_Interact_C"))
  (`UserWidget.AddToViewport` _returnvalue 0)
  (`SceneComponent.SetVisibility` (`self.PointLight`) true false))

(event `self.Box.OnComponentEndOverlap`
  (params (OverlappedComponent :type "PrimitiveComponent Object Reference") (OtherActor :type "Actor Object Reference") (OtherComp :type "PrimitiveComponent Object Reference") (OtherBodyIndex :type Integer))
  (cast `/Game/FirstPerson/Blueprints/BP_FirstPersonCharacter` OtherActor)
  (set `self.IsplayerNear?` false)
  (`Widget.RemoveFromParent` (stale `self.Box.OnComponentBeginOverlap` _returnvalue))
  (`SceneComponent.SetVisibility` (`self.PointLight`) false false))

(event `Key|E` :consume false
  (params (Key :type "Key Structure"))
  (:`Pressed`
    (if (`self.IsplayerNear?`)
      (bind (_direction _newtrack_0) (`Timeline|Timeline` :!label _label)
        (:`Update`
          (`SceneComponent.K2_SetRelativeRotation` (`self.Fridge_Door`) (`KismetMathLibrary.RLerp` (struct) (struct :`Yaw` 90.0) _newtrack_0) false false)
          (`KismetSystemLibrary.Delay` 3.0)
          (`self.CloseDoorFridge`))))))

(event `CloseDoorFridge`
  (goto _label :!via `Reverse`))

(fn `UserConstructionScript`)
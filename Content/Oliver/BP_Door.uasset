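; BP_Door is an interactive door that swings open when the player presses E nearby, then closes automatically.
; A box overlap with BP_FirstPersonCharacter sets a proximity flag and shows or removes the WBP_Interact prompt widget.
; The E key, enabled on the actor at BeginPlay, plays a timeline that lerps the door mesh's rotation.
; A Delay chained to that timeline's Update calls CloseDoor, which reverses the timeline.
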(event `self.ReceiveBeginPlay`
  (`self.EnableInput` (`GameplayStatics.GetPlayerController` 0)))

(event `self.Box.OnComponentBeginOverlap`
  (params (OverlappedComponent :type "PrimitiveComponent Object Reference") (OtherActor :type "Actor Object Reference") (OtherComp :type "PrimitiveComponent Object Reference") (OtherBodyIndex :type Integer) (bFromSweep :type Boolean) (SweepResult :type "HitResult Structure (by ref)"))
  (cast `/Game/FirstPerson/Blueprints/BP_FirstPersonCharacter` OtherActor)
  (set `self.IsPlayerNear?` true)
  (bind _returnvalue (`|CreateWidget` "/Game/Oliver/Widgets/WBP_Interact.WBP_Interact_C"))
  (`UserWidget.AddToViewport` _returnvalue 0))

(event `self.Box.OnComponentEndOverlap`
  (params (OverlappedComponent :type "PrimitiveComponent Object Reference") (OtherActor :type "Actor Object Reference") (OtherComp :type "PrimitiveComponent Object Reference") (OtherBodyIndex :type Integer))
  (cast `/Game/FirstPerson/Blueprints/BP_FirstPersonCharacter` OtherActor)
  (set `self.IsPlayerNear?` false)
  (`Widget.RemoveFromParent` (stale `self.Box.OnComponentBeginOverlap` _returnvalue)))

(event `Key|E` :consume false
  (params (Key :type "Key Structure"))
  (:`Pressed`
    (if (`self.IsPlayerNear?`)
      (bind (_direction _newtrack_0) (`Timeline|Door_T` :!label _label)
        (:`Update`
          (`SceneComponent.K2_SetRelativeRotation` (`self.SM_Door`) (`KismetMathLibrary.RLerp` (struct) (struct :`Yaw` 90.0) _newtrack_0) false false)
          (`KismetSystemLibrary.Delay` 3.0)
          (`self.CloseDoor`))))))

(event `CloseDoor`
  (goto _label :!via `Reverse`))

(fn `UserConstructionScript`)